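; BP_GM is a game manager that drives the level's obstacles, starting both behaviors on BeginPlay.
; A looping one-second timer spawns double-scale BP_SphereObstacle actors using the transforms of randomly picked TargetPoints in the level.
; The SwingTerm timeline moves the first BP_Cylinder found, adding its CylinderLocation track to the actor's current location each update, so the offset accumulates rather than following a fixed origin.
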(event `self.ReceiveBeginPlay`
  (`self.SlideBegin`)
  (`self.SwingCylinder`))

(event `SlideBegin`
  (`KismetSystemLibrary.K2_SetTimerDelegate` (delegate `SlideSphereSpawnEvent`) 1.0 true))

(event `SlideSphereSpawnEvent`
  (bind _outactors (`GameplayStatics.GetAllActorsOfClass` "/Script/Engine.TargetPoint"))
  (bind (_returnvalue_location _returnvalue_rotation) (`KismetMathLibrary.BreakTransform` (`self.GetTransform` (`|GetArrayItem` _outactors (`KismetMathLibrary.RandomIntegerInRange` 0 (- (`KismetArrayLibrary.Array_Length` _outactors) 1))))))
  (`|SpawnActorFromClass` "/Game/Blueprints/BP_SphereObstacle.BP_SphereObstacle_C" (`KismetMathLibrary.MakeTransform` _returnvalue_location _returnvalue_rotation (2.0 2.0 2.0)) "Undefined" "OverrideRootScale" null null))

(event `SwingCylinder`
  (bind _outactors (`GameplayStatics.GetAllActorsOfClass` "/Game/Blueprints/BP_Cylinder.BP_Cylinder_C"))
  (bind (_direction _cylinderlocation) (`Timeline|SwingTerm`)
    (:`Update`
      (bind _output (`|GetArrayItem` _outactors))
      (`self.K2_SetActorRelativeLocation` _output (+ _cylinderlocation (`self.K2_GetActorLocation` _output)) false false))))

(fn `UserConstructionScript`)