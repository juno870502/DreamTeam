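; BP_UpDownTrigger is a camera-switch trigger volume for the BP_TPC third-person character.
; When the character enters the collision component, its player controller blends the view to the first CameraActor found in the level, and SwitchCamera passes that camera to the character.
; On exit, the view blends back to the character and SwitchCamera restores its own camera mode.
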(event `self.ReceiveActorBeginOverlap`
  (params (OtherActor :type "Actor Object Reference")))

(event `self.CollisionComponent.OnComponentBeginOverlap`
  (params (OverlappedComponent :type "PrimitiveComponent Object Reference") (OtherActor :type "Actor Object Reference") (OtherComp :type "PrimitiveComponent Object Reference") (OtherBodyIndex :type Integer) (bFromSweep :type Boolean) (SweepResult :type "HitResult Structure (by ref)"))
  (bind _asbp_tpc (cast `/Game/Blueprints/BP_TPC` OtherActor))
  (bind _asplayer_controller (cast `PlayerController` (`Pawn.GetController` _asbp_tpc)))
  (bind _outactors (`GameplayStatics.GetAllActorsOfClass` "/Script/Engine.CameraActor"))
  (bind _output (`|GetArrayItem` _outactors))
  (`PlayerController.SetViewTargetWithBlend` _asplayer_controller _output 0.5 "VTBlend_Linear" 0.0 false)
  (`/Game/Blueprints/BP_TPC.SwitchCamera` _asbp_tpc false _output))

(event `self.CollisionComponent.OnComponentEndOverlap`
  (params (OverlappedComponent :type "PrimitiveComponent Object Reference") (OtherActor :type "Actor Object Reference") (OtherComp :type "PrimitiveComponent Object Reference") (OtherBodyIndex :type Integer))
  (bind _asbp_tpc (cast `/Game/Blueprints/BP_TPC` OtherActor))
  (bind _asplayer_controller (cast `PlayerController` (`Pawn.GetController` _asbp_tpc)))
  (`PlayerController.SetViewTargetWithBlend` _asplayer_controller _asbp_tpc 0.5 "VTBlend_Linear" 0.0 false)
  (`/Game/Blueprints/BP_TPC.SwitchCamera` _asbp_tpc true null))

(fn `UserConstructionScript`)