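; Player character Blueprint that routes input between normal movement and a ledge climbing component.
; LeftAlt exits a grab and SpaceBar climbs the ledge, both only while hanging.
; While hanging or climbing, sideways input drives movement along the ledge and forward input is only stored; otherwise both axes feed PlayerMovementInput.
; The aim action is an empty stub, and construction just calls the parent.
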(event `Key|LeftAlt`
  (params (Key :type "Key Structure"))
  ;[1 1 1] Climbing Input Control
  (:`Pressed`
    (if (`/Game/DTChar/BP/ClimbingComponent.IsHanging` (`self.ClimbingComponent`))
      (`/Game/DTChar/BP/ClimbingComponent.Exit Grab Event` (`self.ClimbingComponent`)))))

(event `Key|SpaceBar`
  (params (Key :type "Key Structure"))
  ;[1 1 1] Climbing Input Control
  (:`Pressed`
    (if (`/Game/DTChar/BP/ClimbingComponent.IsHanging` (`self.ClimbingComponent`))
      (`/Game/DTChar/BP/ClimbingComponent.Climb Ledge Event` (`self.ClimbingComponent`)))))

(event `InputAxis|MoveForward/Backwards`
  (params (AxisValue :type "Float (single-precision)"))
  (bind _climbingcomponent (`self.ClimbingComponent`))
  ;[1 1 1] Climbing Input Control
  (set `self.ForwardAxisValue` AxisValue)
  (if (not (or (`/Game/DTChar/BP/ClimbingComponent.IsHanging` _climbingcomponent) (`/Game/DTChar/BP/ClimbingComponent.IsClimbingLedge` _climbingcomponent)))
    (`self.PlayerMovementInput` true)))

(event `InputAxis|MoveRight/Left`
  (params (AxisValue :type "Float (single-precision)"))
  (bind _climbingcomponent (`self.ClimbingComponent`))
  ;[1 1 1] Climbing Input Control
  (set `self.RightAxisValue` AxisValue)
  (if (or (`/Game/DTChar/BP/ClimbingComponent.IsHanging` _climbingcomponent) (`/Game/DTChar/BP/ClimbingComponent.IsClimbingLedge` _climbingcomponent))
    (`/Game/DTChar/BP/ClimbingComponent.MoveInLedge` (`self.ClimbingComponent`) AxisValue)
    (else
      (`self.PlayerMovementInput` false))))

(event `InputAction|AimAction`
  (params (Key :type "Key Structure"))
  ;[1 1 1] Climbing Input Control
  (:`Pressed`
    (if true
      _)))

(fn `UserConstructionScript`
  (`parent.UserConstructionScript`))