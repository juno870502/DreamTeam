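; Player character Blueprint with a punch-and-grab action that lets it hang from surfaces in ragdoll and climb-jump off them.
; While the punch montage plays, Tick sphere-traces from both hand sockets, shoving "Launchable" components with an impulse.
; Other hits spawn angular-locked physics constraint actors binding that hand to the hit component, then trigger ragdoll hanging.
; Action releases the hold, while Jump also launches the character upward.
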(event `self.ReceiveTick`
  (params (DeltaSeconds :type "Float (single-precision)"))
  (bind _returnvalue (`SceneComponent.GetSocketLocation` (`self.Mesh`) "LHSocket"))
  (bind _returnvalue_2 (`SceneComponent.GetSocketLocation` (`self.Mesh`) "RHSocket"))
  (`parent.ReceiveTick` DeltaSeconds)
  (if (`self.ActionPressed`)
    (`|ExecutionSequence`
      (:`then_0`
        (bind (_outhit _returnvalue_3) (`KismetSystemLibrary.SphereTraceSingle` :`Start` _returnvalue_2 :`End` (+ _returnvalue_2 (1.0 0.0 0.0)) :`Radius` 20.0 :`TraceChannel` "TraceTypeQuery3" :`DrawDebugType` "ForOneFrame"))
        (if _returnvalue_3
          (bind (_bblockinghit _binitialoverlap _time _distance _location _impactpoint _normal _impactnormal _physmat _hitactor _hitcomponent) (`GameplayStatics.BreakHitResult` _outhit))
          (if (`ActorComponent.ComponentHasTag` _hitcomponent "Launchable")
            (`PrimitiveComponent.AddImpulse` _hitcomponent (* _impactnormal -999999.0) "None" false)
            (else
              (`self.Set Constraint` _location "RHSocket" _hitcomponent)))))
      (:`then_1`
        (bind (_outhit_2 _returnvalue_4) (`KismetSystemLibrary.SphereTraceSingle` :`Start` _returnvalue :`End` (+ _returnvalue (1.0 0.0 0.0)) :`Radius` 20.0 :`TraceChannel` "TraceTypeQuery3" :`DrawDebugType` "ForOneFrame"))
        (if _returnvalue_4
          (bind (_bblockinghit_2 _binitialoverlap_2 _time_2 _distance_2 _location_2 _impactpoint_2 _normal_2 _impactnormal_2 _physmat_2 _hitactor_2 _hitcomponent_2) (`GameplayStatics.BreakHitResult` _outhit_2))
          (if (`ActorComponent.ComponentHasTag` _hitcomponent_2 "Launchable")
            (`PrimitiveComponent.AddImpulse` _hitcomponent_2 (* _impactnormal_2 -999999.0) "None" false)
            (else
              (`self.Set Constraint` _location_2 "LHSocket" _hitcomponent_2))))))))

(event `InputAction|AimAction`
  (params (Key :type "Key Structure"))
  (:`Pressed`
    (if true
      _)))

(event `InputAction|Action`
  (params (Key :type "Key Structure"))
  ;[1 1 1] Action Montage
  (:`Pressed`
    (if (`self.IsHanging`)
      (`self.ReleaseConstraints`)
      (`self.Un_Ragdoll Event`)
      (set `self.IsHanging` false)
      (elif (not (`self.ActionPressed`))
        (set `self.ActionPressed` true)
        (`self.ReleaseConstraints`)
        (`self.Play Action Animation` true)))))

(event `Play Action Animation`
  (params (IsPlay :type Boolean :default true))
  ;[1 1 1] Action Montage
  (if IsPlay
    (`|PlayMontage` (`self.Mesh`) "/Game/DTChar/Anim/Char_Chocho/ActionMontage/PunchMontage.PunchMontage" 1.0 0.0 "Start"
      (:`OnCompleted`
        _)
      (:`OnInterrupted`
        _))
    (else
      (`self.StopAnimMontage` "/Game/DTChar/Anim/Char_Chocho/ActionMontage/PunchMontage.PunchMontage")))
  (set `self.ActionPressed` false))

(event `Set Constraint`
  (params (NewVector :type "Vector Structure") (SocketName :type Name) (TargetComponent :type "PrimitiveComponent Object Reference"))
  ;[1 1 1] Set Constraint
  (switch `name` SocketName
    (:`LHSocket`
      (bind _returnvalue (`|SpawnActorFromClass` "/Script/Engine.PhysicsConstraintActor" (`KismetMathLibrary.MakeTransform` NewVector) "AdjustIfPossibleButDontSpawnIfColliding" "OverrideRootScale" null null))
      (bind _output_get (set `self.LConstraint` _returnvalue))
      (`/Engine/EditorBlueprintResources/StandardMacros.IsValid` _output_get
        (:`Is Valid`
          (bind _constraintcomp (`PhysicsConstraintActor.ConstraintComp` _output_get))
          (`PhysicsConstraintComponent.SetConstrainedComponents` _constraintcomp (`self.Mesh`) "L_Hand" TargetComponent "None")
          (`PhysicsConstraintComponent.SetAngularSwing1Limit` _constraintcomp "ACM_Locked" 0.0)
          (`PhysicsConstraintComponent.SetAngularSwing2Limit` _constraintcomp "ACM_Locked" 0.0)
          (`PhysicsConstraintComponent.SetAngularTwistLimit` _constraintcomp "ACM_Locked" 0.0)
          (`self.To_Ragdoll Event`)
          (set `self.IsHanging` true))))
    (:`RHSocket`
      (bind _returnvalue_2 (`|SpawnActorFromClass` "/Script/Engine.PhysicsConstraintActor" (`KismetMathLibrary.MakeTransform` NewVector) "AdjustIfPossibleButDontSpawnIfColliding" "OverrideRootScale" null null))
      (bind _output_get_2 (set `self.RConstraint` _returnvalue_2))
      (`/Engine/EditorBlueprintResources/StandardMacros.IsValid` _output_get_2
        (:`Is Valid`
          (bind _constraintcomp_2 (`PhysicsConstraintActor.ConstraintComp` _output_get_2))
          (`PhysicsConstraintComponent.SetConstrainedComponents` _constraintcomp_2 (`self.Mesh`) "R_Hand" TargetComponent "None")
          (`PhysicsConstraintComponent.SetAngularSwing1Limit` _constraintcomp_2 "ACM_Locked" 0.0)
          (`PhysicsConstraintComponent.SetAngularSwing2Limit` _constraintcomp_2 "ACM_Locked" 0.0)
          (`PhysicsConstraintComponent.SetAngularTwistLimit` _constraintcomp_2 "ACM_Locked" 0.0)
          (`self.To_Ragdoll Event`)
          (set `self.IsHanging` true))))))

(event `InputAction|JumpAction`
  (params (Key :type "Key Structure"))
  ;[1 1 1] Climb Jump Action
  (:`Pressed`
    (if (`self.IsHanging`)
      (`self.Un_Ragdoll Event`)
      (`self.LaunchCharacter` (0.0 0.0 600.0))
      (`self.ReleaseConstraints`)
      (set `self.IsHanging` false)
      (else
        (`self.Jump`))))
  (:`Released`
    (`self.StopJumping`)))

(event `ReleaseConstraints`
  (bind _rconstraint (`self.RConstraint`))
  (bind _lconstraint (`self.LConstraint`))
  ;[1 1 1] Release Constraints
  (`/Engine/EditorBlueprintResources/StandardMacros.IsValid` _rconstraint
    (:`Is Valid`
      (`self.K2_DestroyActor` _rconstraint))
    (:`Is Not Valid`
      _))
  (`/Engine/EditorBlueprintResources/StandardMacros.IsValid` _lconstraint
    (:`Is Valid`
      (`self.K2_DestroyActor` _lconstraint))))

(fn `UserConstructionScript`
  (`parent.UserConstructionScript`))