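; Button actor for the 3D printer that triggers the printer plate's front-button action.
; On BeginPlay it caches the first BP_3DPrinterPlate found in the level.
; VirtualAction calls PushFrontButton on that plate and, when it returns true, sets the button's emissive color to bright yellow.
; The construction script creates the dynamic instance of the red material used for that color change.
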(event `self.ReceiveBeginPlay`
  (bind _outactors (`GameplayStatics.GetAllActorsOfClass` "/Game/ObjectBP/3DPrinter/BP_3DPrinterPlate.BP_3DPrinterPlate_C"))
  (set `self.3DPrinterPlate` (`|GetArrayItem` _outactors)))

(event `/Game/DTChar/BP/BPI_Action.VirtualAction`
  (bind _lighton (`/Game/ObjectBP/3DPrinter/BP_3DPrinterPlate.PushFrontButton` (`self.3DPrinterPlate`)))
  (if _lighton
    (`MaterialInstanceDynamic.SetVectorParameterValue` (`self.MI_Button`) "EmisiveColor" (struct :`R` 10.0 :`G` 10.0 :`A` 1.0))))

(fn `UserConstructionScript`
  (bind _returnvalue (`PrimitiveComponent.CreateDynamicMaterialInstance` (`self.StaticMesh1`) 0 "/Game/Objects/3D_printer/_Red_._Red_" "None"))
  (set `self.MI_Button` _returnvalue))