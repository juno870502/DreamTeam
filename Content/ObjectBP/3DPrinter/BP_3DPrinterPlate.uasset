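; BP_3DPrinterPlate is the moving plate of a 3D printer, traveling between its original (down) and target (up) locations.
; Two timelines drive UpPlate and DownPlate, lerping from the current location on each update and setting an OnGoing, UpFloor or DownFloor state.
; PushFrontButton lowers a raised plate and returns true when it does so or the plate is already moving.
; VirtualAction calls PushInsideButton, which also branches on that state.
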(event `DownPlate`
  (bind (_direction _time) (`Timeline|OriginalTimeLine` :!via `PlayFromStart`)
    (:`Update`
      (`self.K2_SetActorLocation` (`KismetMathLibrary.VLerp` (`self.K2_GetActorLocation`) (`self.OriginalLocation`) _time))
      (set `self.State` "NewEnumerator1"))
    (:`Finished`
      (set `self.State` "NewEnumerator0"))))

(event `UpPlate`
  (bind (_direction _time) (`Timeline|TargetTimeLine` :!via `PlayFromStart`)
    (:`Update`
      (`self.K2_SetActorLocation` (`KismetMathLibrary.VLerp` (`self.K2_GetActorLocation`) (`self.TargetLocation`) _time))
      (set `self.State` "NewEnumerator1"))
    (:`Finished`
      (set `self.State` "NewEnumerator2"))))

(event `/Game/DTChar/BP/BPI_Action.VirtualAction`
  (`self.PushInsideButton`))

(fn `PushFrontButton`
  (returns (LightOn :type Boolean))
  (switch `/Game/ObjectBP/3DPrinter/PlateStatus` (`self.State`)
    (:`NewEnumerator1`
      _)
    (:`NewEnumerator2`
      (`self.DownPlate`)))
  (return true))

(fn `PushInsideButton`
  (switch `/Game/ObjectBP/3DPrinter/PlateStatus` (`self.State`)))

(fn `UserConstructionScript`)