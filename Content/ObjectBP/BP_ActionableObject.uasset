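; BP_ActionableObject is an actor with a configurable static mesh that gets pushed by a physics impulse when acted upon.
; Its construction script applies NewMesh, creates a dynamic material instance from MI and fills the "Base" vector parameter from a random unit vector, varying each object's look.
; The VirtualAction event applies the incoming vector, scaled by ImpulsePower, as a mass-dependent impulse on the mesh.
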(event `/Game/DTChar/BP/BPI_Action.VirtualAction`
  (params (ImpulseVector :type "Vector Structure"))
  (`PrimitiveComponent.AddImpulse` (`self.StaticMesh`) (* ImpulseVector (`self.ImpulsePower`)) "None" false))

(fn `UserConstructionScript`
  (bind (_returnvalue_x _returnvalue_y _returnvalue_z) (`KismetMathLibrary.BreakVector` (`KismetMathLibrary.RandomUnitVector`)))
  (bind _staticmesh (`self.StaticMesh`))
  (`StaticMeshComponent.SetStaticMesh` _staticmesh (`self.NewMesh`))
  (bind _returnvalue (`PrimitiveComponent.CreateDynamicMaterialInstance` _staticmesh 0 (`self.MI`) "None"))
  (`MaterialInstanceDynamic.SetVectorParameterValue` _returnvalue "Base" (make `LinearColor` _returnvalue_x _returnvalue_y _returnvalue_z 1.0)))