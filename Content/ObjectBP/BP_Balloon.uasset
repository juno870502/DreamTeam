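; BP_Balloon is a balloon actor that sinks in steps after its static mesh is hit.
; BeginPlay records the starting height, and each hit starts a looping half-second timer that moves the actor down by DownVelocity.
; The timer clears its stored handle once the drop exceeds MaxDistance.
; Repeat hits overwrite that handle without clearing the earlier timer.
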(event `self.ReceiveBeginPlay`
  (set `self.InitialZValue` (.z (`self.K2_GetActorLocation`))))

(event `self.StaticMeshComponent.OnComponentHit`
  (params (HitComponent :type "PrimitiveComponent Object Reference") (OtherActor :type "Actor Object Reference") (OtherComp :type "PrimitiveComponent Object Reference") (NormalImpulse :type "Vector Structure") (Hit :type "HitResult Structure (by ref)"))
  (bind _returnvalue (`KismetSystemLibrary.K2_SetTimerDelegate` (delegate `MoveDown`) 0.5 true))
  (set `self.TimerHandle` _returnvalue))

(event `self.StaticMeshComponent.OnComponentBeginOverlap`
  (params (OverlappedComponent :type "PrimitiveComponent Object Reference") (OtherActor :type "Actor Object Reference") (OtherComp :type "PrimitiveComponent Object Reference") (OtherBodyIndex :type Integer) (bFromSweep :type Boolean) (SweepResult :type "HitResult Structure (by ref)")))

(event `MoveDown`
  (bind (_returnvalue_x _returnvalue_y _returnvalue_z) (`KismetMathLibrary.BreakVector` (`self.K2_GetActorLocation`)))
  (`self.K2_AddActorWorldOffset` (`KismetMathLibrary.MakeVector` 0.0 0.0 (* -1 (`self.DownVelocity`))))
  (if (> (- (`self.InitialZValue`) _returnvalue_z) (`self.MaxDistance`))
    (`KismetSystemLibrary.K2_ClearAndInvalidateTimerHandle` (`self.TimerHandle`))))

(fn `UserConstructionScript`)