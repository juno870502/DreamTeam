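; Game manager Blueprint (BP_GM) for an obstacle course, holding hazard events, a record timer and checkpoint state.
; BeginSlide repeatedly spawns sphere obstacles at random TargetPoints, and BeginSwingCylinder moves two cylinders oppositely via a timeline.
; SavePoint stores the latest checkpoint and respawn vector, turning other save point lights red.
; BeginPlay is empty, and the local calls starting hazards and the seconds-printing timer are disconnected.
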(event `self.ReceiveBeginPlay`)

(event `RecoredTimer`
  (bind _result (`/Engine/EditorBlueprintResources/StandardMacros.IncrementInt` (`self.RecordTimer`))
    (:`  `
      (`KismetSystemLibrary.PrintString` (`KismetStringLibrary.Conv_IntToString` _result)))))

(event `BeginSlide`
  ;[1 1 1] Slide Sphere
  (`KismetSystemLibrary.K2_SetTimerDelegate` (delegate `SlideSphereSpawnEvent`) 1.0 true))

(event `SlideSphereSpawnEvent`
  ;[1 1 1] Slide Sphere
  (bind _outactors (`GameplayStatics.GetAllActorsOfClass` "/Script/Engine.TargetPoint"))
  (bind (_returnvalue_location _returnvalue_rotation) (`KismetMathLibrary.BreakTransform` (`self.GetTransform` (`|GetArrayItem` _outactors (`KismetMathLibrary.RandomIntegerInRange` 0 (- (`KismetArrayLibrary.Array_Length` _outactors) 1))))))
  (`|SpawnActorFromClass` "/Game/ObjectBP/BP_SphereObstacle.BP_SphereObstacle_C" (`KismetMathLibrary.MakeTransform` _returnvalue_location _returnvalue_rotation (2.0 2.0 2.0)) "Undefined" "OverrideRootScale" null null))

(event `BeginSwingCylinder`
  ;[1 1 1] Swing Cylinder
  (bind _outactors (`GameplayStatics.GetAllActorsOfClass` "/Game/ObjectBP/BP_Cylinder.BP_Cylinder_C"))
  (bind (_direction _cylinderlocation) (`Timeline|SwingTerm`)
    (:`Update`
      (`|ExecutionSequence`
        (:`then_0`
          (bind _output (`|GetArrayItem` _outactors))
          (`self.K2_SetActorRelativeLocation` _output (+ _cylinderlocation (`self.K2_GetActorLocation` _output)) false false))
        (:`then_1`
          (bind _output_2 (`|GetArrayItem` _outactors 1))
          (`self.K2_SetActorRelativeLocation` _output_2 (+ (* _cylinderlocation -1.0) (`self.K2_GetActorLocation` _output_2)) false false))))))

(event `/Game/ObjectBP/Logic/BPI_Save.SavePoint`
  (params (SavePointVector :type "Vector Structure") (SavePoint :type "/Game/ObjectBP/BP_SavePoint Object Reference"))
  (set `self.LastSavePoint` SavePoint)
  (set `self.RespawnVector` SavePointVector)
  (bind _outactors (`GameplayStatics.GetAllActorsOfClass` "/Game/ObjectBP/BP_SavePoint.BP_SavePoint_C"))
  (for _array_element _outactors
    (if (!= _array_element (`self.LastSavePoint`))
      (`LightComponent.SetLightColor` (`/Game/ObjectBP/BP_SavePoint.PointLight` _array_element) (struct :`R` 1.0 :`A` 1.0) true))))

(fn `UserConstructionScript`)