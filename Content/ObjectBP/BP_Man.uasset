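; BP_Man is a watchman actor that replays a patrol animation and signals pawn sightings with its spotlight color.
; A looping timer set on BeginPlay plays Man_Anim once every Cycle interval.
; StartPawnSensing and EndPawnSensing, not called within this graph, toggle CanSeePawn.
; PawnSensing still fires when the flag is off, so each sighting turns the light red or green according to CanSeePawn.
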(event `self.ReceiveBeginPlay`
  (`KismetSystemLibrary.K2_SetTimerDelegate` (delegate `Patrol`) (`self.Cycle`) true))

(event `Patrol`
  (`SkeletalMeshComponent.PlayAnimation` (`self.SkeletalMesh`) "/Game/Objects/Man/man_Anim.man_Anim" false))

(event `StartPawnSensing`
  (set `self.CanSeePawn` true))

(event `EndPawnSensing`
  (set `self.CanSeePawn` false))

(event `self.PawnSensing.OnSeePawn`
  (params (Pawn :type "Pawn Object Reference"))
  (if (`self.CanSeePawn`)
    (`LightComponent.SetLightColor` (`self.SpotLight`) (struct :`R` 1.0 :`A` 1.0) true)
    (else
      (`LightComponent.SetLightColor` (`self.SpotLight`) (struct :`G` 1.0 :`A` 1.0) true))))

(fn `UserConstructionScript`)