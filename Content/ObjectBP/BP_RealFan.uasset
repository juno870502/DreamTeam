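; BP_RealFan is a fan Blueprint that pushes characters standing in its airflow along an arrow's forward direction.
; Each Tick it sphere-traces from the Arrow over a set Length and Radius and stores any hit Character.
; By default logic it adds continuous movement force scaled by Power; with IsOnce set, it applies a single impulse through a DoOnce that is never reset.
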(event `self.ReceiveTick`
  (params (DeltaSeconds :type "Float (single-precision)"))
  (bind _arrow (`self.Arrow`))
  (bind _returnvalue (`SceneComponent.K2_GetComponentLocation` _arrow))
  (bind (_outhit _returnvalue_2) (`KismetSystemLibrary.SphereTraceSingle` _returnvalue (+ _returnvalue (* (`SceneComponent.GetForwardVector` _arrow) (`self.Length`))) (`self.Radius`) "TraceTypeQuery4"))
  (if _returnvalue_2
    (bind _ascharacter (cast `Character` (`.HitActor` (`GameplayStatics.BreakHitResult` _outhit))))
    (set `self.OverlapCharacter` _ascharacter)
    (if (`self.IsOnce`)
      (`/Engine/EditorBlueprintResources/StandardMacros.DoOnce` false
        (:`Completed`
          (`CharacterMovementComponent.AddImpulse` (`Character.CharacterMovement` (`self.OverlapCharacter`)) (* (`SceneComponent.GetForwardVector` (`self.Arrow`)) (`self.Power`)) false)))
      (else
        (`CharacterMovementComponent.AddForce` (`Character.CharacterMovement` (`self.OverlapCharacter`)) (* (`SceneComponent.GetForwardVector` (`self.Arrow`)) (`self.Power`)))))))

(fn `UserConstructionScript`)