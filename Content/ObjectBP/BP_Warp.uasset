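; BP_Warp is a teleporter actor that moves any overlapping actor to the location of its linked OutWarp.
; On begin overlap, if CanTeleport is true, it disables teleporting on OutWarp, plays a warp sound and sets the actor's location without sweep.
; End overlap re-enables CanTeleport, so the arriving actor is not bounced back until it leaves the destination.
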(event `self.ReceiveActorBeginOverlap`
  (params (OtherActor :type "Actor Object Reference"))
  (if (`self.CanTeleport`)
    (set `/Game/ObjectBP/BP_Warp.CanTeleport` false (`self.OutWarp`))
    (`GameplayStatics.PlaySoundAtLocation` "/Game/GAME_SOUND/SC_Warp.SC_Warp" (`self.K2_GetActorLocation`) (struct) 1.0 1.0 0.0 null null null)
    (`self.K2_SetActorLocation` OtherActor (`self.K2_GetActorLocation` (`self.OutWarp`)) false false)))

(event `self.ReceiveActorEndOverlap`
  (params (OtherActor :type "Actor Object Reference"))
  (if (not (`self.CanTeleport`))
    (set `self.CanTeleport` true)))

(fn `UserConstructionScript`)