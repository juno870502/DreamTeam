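; BP_Merged_Plate is an obstacle plate that moves between OriginalLocation and TargetLocation when a Character enters its Box.
; Each overlap stops both timelines, then sends the plate to OriginalLocation if its Z is above the two locations' midpoint, otherwise to TargetLocation.
; The chosen timeline lerps from the current location each update rather than a cached start, so motion compounds and is non-linear.
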(event `OriginalPlate`
  (bind (_direction _time) (`Timeline|OriginalTimeLine` :!via `PlayFromStart`)
    (:`Update`
      (`self.K2_SetActorLocation` (`KismetMathLibrary.VLerp` (`self.K2_GetActorLocation`) (`self.OriginalLocation`) _time)))))

(event `TargetPlate`
  (bind (_direction _time) (`Timeline|TargetTimeLine` :!via `PlayFromStart`)
    (:`Update`
      (`self.K2_SetActorLocation` (`KismetMathLibrary.VLerp` (`self.K2_GetActorLocation`) (`self.TargetLocation`) _time)))))

(event `self.Box.OnComponentBeginOverlap`
  (params (OverlappedComponent :type "PrimitiveComponent Object Reference") (OtherActor :type "Actor Object Reference") (OtherComp :type "PrimitiveComponent Object Reference") (OtherBodyIndex :type Integer) (bFromSweep :type Boolean) (SweepResult :type "HitResult Structure (by ref)"))
  (cast `Character` OtherActor)
  (`TimelineComponent.Stop` (`self.TargetTimeLine`))
  (`TimelineComponent.Stop` (`self.OriginalTimeLine`))
  (if (> (.z (`self.K2_GetActorLocation`)) (* (+ (.z (`self.OriginalLocation`)) (.z (`self.TargetLocation`))) 0.5))
    (`self.OriginalPlate`)
    (else
      (`self.TargetPlate`))))

(fn `UserConstructionScript`)