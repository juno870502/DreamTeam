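; BP_Pan is a fan-like obstacle that pushes characters along its forward vector.
; Every Tick it runs a debug-drawn sphere trace on the Camera channel, sized by Length and Radius, and stores any character hit.
; With IsOnce set, it applies a Power-scaled impulse through a DoOnce that is never reset; otherwise it adds continuous force to the character's movement component on each hit frame.
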(event `self.ReceiveTick`
  (params (DeltaSeconds :type "Float (single-precision)"))
  (bind _returnvalue (`self.K2_GetActorLocation`))
  (bind (_outhit _returnvalue_2) (`KismetSystemLibrary.SphereTraceSingle` :`Start` _returnvalue :`End` (+ _returnvalue (* (`self.GetActorForwardVector`) (`self.Length`))) :`Radius` (`self.Radius`) :`TraceChannel` "TraceTypeQuery2" :`DrawDebugType` "ForOneFrame"))
  (if _returnvalue_2
    (bind _ascharacter (cast `Character` (`.HitActor` (`GameplayStatics.BreakHitResult` _outhit))))
    (set `self.OverlapCharacter` _ascharacter)
    (if (`self.IsOnce`)
      (`/Engine/EditorBlueprintResources/StandardMacros.DoOnce` false
        (:`Completed`
          (`self.AddImpulse`)))
      (else
        (`self.AddForce`)))))

(fn `AddForce`
  (`CharacterMovementComponent.AddForce` (`Character.CharacterMovement` (`self.OverlapCharacter`)) (* (`self.GetActorForwardVector`) (`self.Power`))))

(fn `AddImpulse`
  (`CharacterMovementComponent.AddImpulse` (`Character.CharacterMovement` (`self.OverlapCharacter`)) (* (`self.GetActorForwardVector`) (`self.Power`)) false))

(fn `UserConstructionScript`)